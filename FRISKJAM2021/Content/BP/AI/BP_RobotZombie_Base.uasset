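; BP_RobotZombie_Base is a robot zombie base Blueprint that plays a melee-style attack animation while the player is within its trigger.
; OverlapTrigger begin and end events track whether the player pawn is inside through an Overlapping flag.
; The attack montage replays whenever it completes or is interrupted while that flag is set, forming a loop.
; The graph applies no damage and contains no movement logic.
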(event OnComponentBeginOverlap(OverlapTrigger)
  (params (OverlappedComponent :type Primitive%20Component%20Object%20Reference) (OtherActor :type Actor%20Object%20Reference) (OtherComp :type Primitive%20Component%20Object%20Reference) (OtherBodyIndex :type Integer) (bFromSweep :type Boolean) (SweepResult :type Hit%20Result%20Structure%20%28by%20ref%29))
  (if (== OtherActor (Game|Player|GetPlayerPawn 0)) :!label _label
    (Variables|Default|SetOverlapping true)
    (Animation|Montage|PlayMontage (Variables|Character|GetMesh) "/Game/ZombieRobot/ZombieRobot/Montage_RobotZombieAttack2.Montage_RobotZombieAttack2"
      (:OnCompleted
        _)
      (:OnInterrupted
        _))
    (if (Variables|Default|GetOverlapping)
      (goto _label))))

(event OnComponentEndOverlap(OverlapTrigger)
  (params (OverlappedComponent :type Primitive%20Component%20Object%20Reference) (OtherActor :type Actor%20Object%20Reference) (OtherComp :type Primitive%20Component%20Object%20Reference) (OtherBodyIndex :type Integer))
  (if (== OtherActor (Game|Player|GetPlayerPawn 0))
    (Variables|Default|SetOverlapping false)))

(event EventBeginPlay)

(fn ConstructionScript)