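; BP_Child is a projectile actor that the player must catch, ending the game if it is missed.
; Overlapping BP_Player with its Collision calls CatchChild and destroys the actor.
; Tick triggers GameOver on GM_FriskJam2021 once the child trails the player by over 50 units on world Y.
; The construction script sets projectile speed from InitialSpeed, and stopping swaps in the KoaraBwait mesh and plays its animation once.
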(event OnProjectileStop(ProjectileMovement)
  (params (ImpactResult :type Hit%20Result%20Structure%20%28by%20ref%29))
  (bind _skeletalmesh (Variables|Default|GetSkeletalMesh))
  (Class|SkinnedMeshComponent|SetSkeletalMesh _skeletalmesh "/Game/Player/Meshes/KoaraB/Wait/KoaraBwait.KoaraBwait" true)
  (Components|Animation|PlayAnimation _skeletalmesh "/Game/Player/Meshes/KoaraB/Wait/KoaraBwait_Anim.KoaraBwait_Anim" false))

(event OnComponentBeginOverlap(Collision)
  (params (OverlappedComponent :type Primitive%20Component%20Object%20Reference) (OtherActor :type Actor%20Object%20Reference) (OtherComp :type Primitive%20Component%20Object%20Reference) (OtherBodyIndex :type Integer) (bFromSweep :type Boolean) (SweepResult :type Hit%20Result%20Structure%20%28by%20ref%29))
  (bind _asbp_player (Utilities|Casting|CastToBP_Player OtherActor))
  (Default|CatchChild _asbp_player)
  (Actor|DestroyActor))

(event EventBeginPlay)

(event Collision|EventActorBeginOverlap
  (params (OtherActor :type Actor%20Object%20Reference)))

(event EventTick
  (params (DeltaSeconds :type Float%20%28single-precision%29))
  (if (< (+ (.y (Transformation|GetActorLocation)) 5e+01) (.y (Transformation|GetActorLocation (Game|GetPlayerCharacter 0))))
    (bind _asgm_frisk_jam_2021 (Utilities|Casting|CastToGM_FriskJam2021 (Game|GetGameMode)))
    (Default|GameOver _asgm_frisk_jam_2021)))

(fn ConstructionScript
  (Variables|/Script/Engine.ProjectileMovementComponent|SetInitialSpeed (Variables|Default|GetProjectileMovement) (Variables|Default|GetInitial%20Speed)))