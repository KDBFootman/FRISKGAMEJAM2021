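; Player pawn for a Frisk Jam 2021 game that auto-advances along Y, steers sideways and can carry and throw a child.
; HP drains over time, faster while carrying, when movement is also slower; running out calls GameOver on the game mode.
; Space jumps, or when carrying charges throw power up to a cap and spawns a thrown Child on release.
; CatchChild and HealHP handle pickup and clamped healing.
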(event EventBeginPlay
  (Input|SetInputModeGameOnly (Game|GetPlayerController 0))
  (Variables|Default|Setthrow_power (Variables|Default|Getthrow_power_init))
  (bind _returnvalue (UserInterface|CreateWidget "/Game/Player/WBP_HPBar.WBP_HPBar_C"))
  (UserInterface|Viewport|AddtoViewport _returnvalue 0))

(event Collision|EventActorBeginOverlap
  (params (OtherActor :type Actor%20Object%20Reference)))

(event EventTick
  (params (DeltaSeconds :type Float%20%28single-precision%29))
  (if (Variables|Default|GethaveChild)
    (Variables|Default|Setspeed 75.0)
    (else
      (Variables|Default|Setspeed 1.5e+02)))
  (Pawn|Input|AddMovementInput (Math|Vector|MakeVector (* DeltaSeconds (Input|AxisValues|GetMoveRight) (Variables|Default|Getspeed) -1.0) (* DeltaSeconds (Variables|Default|Getstage_speed)) 0.0) 1.0 false)
  (if (Variables|Default|GethaveChild)
    (Variables|Default|SetHP_DecreaseSpeed 0.15)
    (else
      (Variables|Default|SetHP_DecreaseSpeed 0.05)))
  (bind _output_get (Variables|Default|SetHP (- (Variables|Default|GetHP) (* (Utilities|Time|GetWorldDeltaSeconds) (Variables|Default|GetHP_DecreaseSpeed)))))
  (if (> _output_get 0.0)
    (if (Variables|Default|GetIsSpacePressed)
      (bind _output_get_2 (Variables|Default|Setthrow_power (+ (Variables|Default|Getthrow_power) (* (Utilities|Time|GetWorldDeltaSeconds) 4e+02))))
      (if (> _output_get_2 (Variables|Default|Getthrow_power_Max))
        (Variables|Default|Setthrow_power (Variables|Default|Getthrow_power_Max)))
      (Development|PrintString (Utilities|String|ToString(Float) (Variables|Default|Getthrow_power)) true true "(R=0.000000,G=0.660000,B=1.000000,A=1.000000)" 0.2))
    (else
      (bind _asgm_frisk_jam_2021 (Utilities|Casting|CastToGM_FriskJam2021 (Game|GetGameMode)))
      (Default|GameOver _asgm_frisk_jam_2021))))

(event Input|ActionEvents|InputActionSpace
  (params (Key :type Key%20Structure :default "None"))
  (bind _returnvalue (Transformation|GetActorTransform))
  (:Pressed
    (if (Variables|Default|GethaveChild)
      (Variables|Default|SetIsSpacePressed true)
      (Variables|Default|Setthrow_power (Variables|Default|Getthrow_power_init))
      (else
        (Character|Jump))))
  (:Released
    (Variables|Default|SetIsSpacePressed false)
    (if (Variables|Default|GethaveChild)
      (Game|SpawnActorfromClass (Variables|Default|GetChild) (Math|Transform|MakeTransform (+ (.location _returnvalue) "0.000000,150.000000, 0") (.rotation _returnvalue) (.scale _returnvalue)) "AdjustIfPossibleButAlwaysSpawn" 0 (Variables|Default|Getthrow_power) 0)
      (Audio|PlaySound2D "/Game/Sounds/SE_Throw.SE_Throw" 1.0 1.0 0.0 0 0)
      (Variables|Default|SethaveChild false)
      (Rendering|SetVisibility (Variables|Default|GetChildMesh) false false))))

(fn ConstructionScript)

(fn HealHP
  (params (heal :type Float%20%28single-precision%29))
  (bind _output_get (Variables|Default|SetHP (+ heal (Variables|Default|GetHP))))
  (if (> _output_get 1.0)
    (Variables|Default|SetHP 1.0))
  (return))

(fn CatchChild
  (Variables|Default|SethaveChild true)
  (Rendering|SetVisibility (Variables|Default|GetChildMesh) true false)
  (Development|PrintString "Catch Child" true true "(R=0.000000,G=0.000000,B=0.000000,A=1.000000)" 1.0)
  (return))